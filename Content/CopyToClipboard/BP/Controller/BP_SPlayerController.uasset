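; BP_SPlayerController is a player controller that tests mock copy-to-clipboard calls for images and textures.
; BeginPlay creates a WBP_UI widget for status feedback.
; Z calls MockCopyImage and reports the red image copy or failure from its result, while X calls MockCopyTexture and always reports success through a hardcoded true condition.
; Both keys print their letter and show the widget for a short delay before removing it.
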(event EventBeginPlay
  (bind _returnvalue (UserInterface|CreateWidget "/Game/CopyToClipboard/UI/WBP_UI.WBP_UI_C" self))
  (Variables|Default|Setwidget _returnvalue))

(event EventTick
  (params (DeltaSeconds :type Float%20%28single-precision%29)))

(event Input|KeyboardEvents|Z
  (params (Key :type Key%20Structure :default "None"))
  (bind _widget (Variables|Default|Getwidget))
  (bind _maintext (Variables|/Game/CopyToClipboard/UI/WBP_UI.WBP_UI_C|GetmainText _widget))
  (:Pressed
    (Development|PrintText "Z")
    (bind _returnvalue (Class|SPlayerController|MockCopyImage))
    (if _returnvalue
      (Variables|/Script/UMG.TextBlock|SetText _maintext "Copied Red Image")
      (else
        (Variables|/Script/UMG.TextBlock|SetText _maintext "Fail")))
    (UserInterface|Viewport|AddtoViewport _widget 0)
    (Utilities|FlowControl|Delay 1.5)
    (Widget|RemovefromParent (Variables|Default|Getwidget))))

(event Input|KeyboardEvents|X
  (params (Key :type Key%20Structure :default "None"))
  (bind _widget (Variables|Default|Getwidget))
  (bind _maintext (Variables|/Game/CopyToClipboard/UI/WBP_UI.WBP_UI_C|GetmainText _widget))
  (:Pressed
    (Development|PrintText "X")
    (Class|SPlayerController|MockCopyTexture)
    (if true
      (Variables|/Script/UMG.TextBlock|SetText _maintext "Copied Texture")
      (else
        (Variables|/Script/UMG.TextBlock|SetText _maintext "Fail")))
    (UserInterface|Viewport|AddtoViewport _widget 0)
    (Utilities|FlowControl|Delay 1.5)
    (Widget|RemovefromParent (Variables|Default|Getwidget))))

(fn ConstructionScript)